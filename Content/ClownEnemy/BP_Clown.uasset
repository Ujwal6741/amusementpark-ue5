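; BP_Clown is a clown boss enemy that chases and attacks the player.
; Pawn sensing triggers AI move-to, while Tick constantly yaws the actor toward the player and, when a living player is inside the AttackRange overlap, plays an attack montage and applies damage on a cooldown.
; Damage drains boss health until a death montage plays and disables chasing and attacking.
; A callable intro freezes movement during a jump montage, restoring walking afterward.
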(event `OnMontageEnded_Event_0`
  (params (Montage :type "AnimMontage Object Reference") (bInterrupted :type Boolean))
  (`CharacterMovementComponent.SetMovementMode` (`self.CharacterMovement`) "MOVE_Walking" 0))

(event `PlayBossIntro`
  (bind _returnvalue (`SkeletalMeshComponent.GetAnimInstance` (`self.Mesh`)))
  (`CharacterMovementComponent.DisableMovement` (`self.CharacterMovement`))
  (`AnimInstance.Montage_Play` _returnvalue "/Game/ClownEnemy/project-playtime-boxy-clown/source/BOXYCLOWNSK_BoxyBoo_Clown_A_Boxy_JumpAbilityAirborne_SK_BoxyBoo_Clown_Montage.BOXYCLOWNSK_BoxyBoo_Clown_A_Boxy_JumpAbilityAirborne_SK_BoxyBoo_Clown_Montage" 1.0 "MontageLength" 0.0 true)
  (add `AnimInstance.OnMontageEnded` _returnvalue (delegate `OnMontageEnded_Event_0`)))

(event `self.PawnSensing.OnSeePawn`
  (params (Pawn :type "Pawn Object Reference"))
  (if (`self.CanChasePlayer`)
    (`|AIMoveTo` self (0.0 0.0 0.0) Pawn)))

(event `self.ReceiveBeginPlay`
  (set `self.CanChasePlayer` true))

(event `self.ReceiveTick`
  (params (DeltaSeconds :type "Float (single-precision)"))
  (`|ExecutionSequence`
    (:`then_0`
      (`self.K2_SetActorRotation` (`KismetMathLibrary.MakeRotator` 0.0 0.0 (- (.yaw (`KismetMathLibrary.FindLookAtRotation` (`self.K2_GetActorLocation`) (`self.K2_GetActorLocation` (`GameplayStatics.GetPlayerCharacter` 0)))) 90.0))))
    (:`then_1`
      (`/Engine/EditorBlueprintResources/StandardMacros.IsValid` (`self.PlayerInRange`)
        (:`Is Valid`
          (if (`/Game/ThirdPerson/Blueprints/BP_ThirdPersonCharacter.IsDead` (`self.PlayerInRange`))
            _
            (elif (`self.CanAttack`)
              (`self.PlayAnimMontage` "/Game/ClownEnemy/project-playtime-boxy-clown/source/Attack.Attack")
              (`GameplayStatics.ApplyDamage` (stale `self.AttackRange.OnComponentBeginOverlap` _asbp_third_person_character) 15.0 null self)
              (set `self.CanAttack` false)
              (`KismetSystemLibrary.Delay` 2.0)
              (set `self.CanAttack` true))))))))

(event `self.AttackRange.OnComponentBeginOverlap`
  (params (OverlappedComponent :type "PrimitiveComponent Object Reference") (OtherActor :type "Actor Object Reference") (OtherComp :type "PrimitiveComponent Object Reference") (OtherBodyIndex :type Integer) (bFromSweep :type Boolean) (SweepResult :type "HitResult Structure (by ref)"))
  (bind _asbp_third_person_character (cast `/Game/ThirdPerson/Blueprints/BP_ThirdPersonCharacter` OtherActor))
  (set `self.PlayerInRange` _asbp_third_person_character))

(event `self.AttackRange.OnComponentEndOverlap`
  (params (OverlappedComponent :type "PrimitiveComponent Object Reference") (OtherActor :type "Actor Object Reference") (OtherComp :type "PrimitiveComponent Object Reference") (OtherBodyIndex :type Integer))
  (set `self.PlayerInRange` null))

(event `self.ReceiveAnyDamage`
  (params (Damage :type "Float (single-precision)") (DamageType :type "DamageType Object Reference") (InstigatedBy :type "Controller Object Reference") (DamageCauser :type "Actor Object Reference"))
  (`KismetSystemLibrary.PrintString` "Hit")
  (set `self.BossHealth` (- (`self.BossHealth`) Damage))
  (if (<= (`self.BossHealth`) 0.0)
    (set `self.CanAttack` false)
    (set `self.CanChasePlayer` false)
    (`self.PlayAnimMontage` "/Game/ClownEnemy/project-playtime-boxy-clown/source/Death.Death")))

(fn `UserConstructionScript`)