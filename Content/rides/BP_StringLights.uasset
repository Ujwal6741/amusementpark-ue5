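; BP_StringLights is a construction-time actor that builds a string of light props along a spline.
; The Construction Script steps along the spline at fixed distance intervals, adding a static mesh and a point light component at each step.
; Only each mesh is moved to its spline point; the point lights receive no location in the script.
; The event graph holds no active logic.
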(fn `UserConstructionScript`
  (for _index (range (+ (`KismetMathLibrary.FTrunc` (/ (`SplineComponent.GetSplineLength` (`self.Spline`)) 50.0)) 1))
    (bind _returnvalue (`AddComponent|NODE_AddStaticMeshComponent-0`))
    (`AddComponent|NODE_AddPointLightComponent-0`)
    (`SceneComponent.K2_SetWorldLocation` _returnvalue (`SplineComponent.GetLocationAtDistanceAlongSpline` (`self.Spline`) (`KismetMathLibrary.Conv_IntToDouble` (* _index 50)) "World") false false)))