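; BP_Carousel is a carousel ride that comes to life when something overlaps its LightTrigger volume.
; The overlap starts a looping spin animation on the carousel mesh, raises the intensity of its eight lights and plays a male laugh sound at the world origin.
; The trigger has no actor filter, one-shot guard or end-overlap reset, so each new overlap repeats the whole sequence.
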(event `self.LightTrigger.OnComponentBeginOverlap`
  (params (OverlappedComponent :type "PrimitiveComponent Object Reference") (OtherActor :type "Actor Object Reference") (OtherComp :type "PrimitiveComponent Object Reference") (OtherBodyIndex :type Integer) (bFromSweep :type Boolean) (SweepResult :type "HitResult Structure (by ref)"))
  (`SkeletalMeshComponent.PlayAnimation` (`self.CarousselMesh`) "/Game/rides/carousel-spinning/source/carousel_spinning/SkeletalMeshes/carousel_spinning_Anim.carousel_spinning_Anim" true)
  (`LightComponent.SetIntensity` (`self.light8`) 10000.0)
  (`LightComponent.SetIntensity` (`self.light1`) 10000.0)
  (`LightComponent.SetIntensity` (`self.light2`) 10000.0)
  (`LightComponent.SetIntensity` (`self.light3`) 10000.0)
  (`LightComponent.SetIntensity` (`self.light4`) 10000.0)
  (`LightComponent.SetIntensity` (`self.light7`) 10000.0)
  (`LightComponent.SetIntensity` (`self.light6`) 10000.0)
  (`LightComponent.SetIntensity` (`self.light5`) 10000.0)
  (`GameplayStatics.PlaySoundAtLocation` "/Game/Audio/universfield-male-laugh-242216.universfield-male-laugh-242216" (0.0 0.0 0.0) (struct) 1.0 1.0 0.0 null null null null))

(fn `UserConstructionScript`)