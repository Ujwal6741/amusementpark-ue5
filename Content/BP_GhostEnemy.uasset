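; Ghost enemy character that chases and attacks the player when seen.
; PawnSensing sets a two-second sight flag, which Tick uses to move toward the player or attack within range.
; Attacks stop movement, focus the player and play a montage and sound on a cooldown, with no damage applied in this graph.
; Damage lowers health; death increments the player's kill count, disables collision and destroys the actor after a delay.
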(event `self.ReceiveBeginPlay`
  (`|ExecutionSequence`
    (:`then_0`
      (if (`self.CanSeePlayer`)
        (`|AIMoveTo` self (0.0 0.0 0.0) (`GameplayStatics.GetPlayerCharacter` 0) 60.0)))
    (:`then_1`
      (set `self.Health` (`self.MaxHealth`)))))

(event `self.ReceiveAnyDamage`
  (params (Damage :type "Float (single-precision)") (DamageType :type "DamageType Object Reference") (InstigatedBy :type "Controller Object Reference") (DamageCauser :type "Actor Object Reference"))
  (`GameplayStatics.PlaySoundAtLocation` "/Game/Audio/freesound_community-hit-swing-sword-small-2-95566.freesound_community-hit-swing-sword-small-2-95566" (`self.K2_GetActorLocation`) (struct) 1.0 1.0 0.0 null null null null)
  (bind _output_get (set `self.Health` (- (`self.Health`) Damage)))
  (if (<= _output_get 0.0)
    (bind _asbp_third_person_character (cast `/Game/ThirdPerson/Blueprints/BP_ThirdPersonCharacter` (`GameplayStatics.GetPlayerCharacter` 0)))
    (bind _output_get_2 (set `/Game/ThirdPerson/Blueprints/BP_ThirdPersonCharacter.EnemiesKilled` (+ (`/Game/ThirdPerson/Blueprints/BP_ThirdPersonCharacter.EnemiesKilled` _asbp_third_person_character) 1) _asbp_third_person_character))
    (`KismetSystemLibrary.PrintString` (`KismetStringLibrary.Conv_IntToString` _output_get_2))
    (set `self.IsDead` true)
    (`MovementComponent.StopMovementImmediately` (`self.CharacterMovement`))
    (`self.SetActorEnableCollision` false)
    (`KismetSystemLibrary.Delay` 2.0)
    (`self.K2_DestroyActor`)))

(event `self.ReceiveTick`
  (params (DeltaSeconds :type "Float (single-precision)"))
  (`|ExecutionSequence`
    (:`then_0`
      (if (`self.CanSeePlayer`)
        (if (< (`self.GetDistanceTo` (`GameplayStatics.GetPlayerCharacter` 0)) (`self.AttackRange`))
          (`self.AttackPlayer`)
          (else
            (`|AIMoveTo` self (0.0 0.0 0.0) (`GameplayStatics.GetPlayerCharacter` 0) 60.0)))))
    (:`then_1`
      (bind _asbp_third_person_character (cast `/Game/ThirdPerson/Blueprints/BP_ThirdPersonCharacter` (`GameplayStatics.GetPlayerCharacter` 0))))))

(event `AttackPlayer`
  (if (and (`self.CanAttack`) (not (`/Game/ThirdPerson/Blueprints/BP_ThirdPersonCharacter.IsDead` (stale `self.ReceiveTick` _asbp_third_person_character))))
    (`MovementComponent.StopMovementImmediately` (`self.CharacterMovement`))
    (bind _asaicontroller (cast `AIController` (`self.GetController`)))
    (`AIController.K2_SetFocus` _asaicontroller (`GameplayStatics.GetPlayerCharacter` 0))
    (`self.PlayAnimMontage` "/Game/Whisper/Animations/AM_Whisper_Attack.AM_Whisper_Attack")
    (`GameplayStatics.PlaySoundAtLocation` "/Game/Audio/freesound_community-monster-attack-47786.freesound_community-monster-attack-47786" (`self.K2_GetActorLocation`) (struct) 1.0 1.0 0.0 null null null null)
    (set `self.CanAttack` false)
    (`KismetSystemLibrary.Delay` (`self.AttackCooldown`))
    (set `self.CanAttack` true)))

(event `self.PawnSensing.OnSeePawn`
  (params (Pawn :type "Pawn Object Reference"))
  (set `self.CanSeePlayer` true)
  (`KismetSystemLibrary.Delay` 2.0)
  (set `self.CanSeePlayer` false))

(fn `UserConstructionScript`)