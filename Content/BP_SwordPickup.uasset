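; BP_SwordPickup is a sword the third-person character picks up and then uses to damage ghost and clown enemies.
; Overlapping its sphere snaps the sword mesh to the character's SwordSocket, stores a reference on the character and sets HasSword.
; The SwordHitbox applies fixed damage to overlapped BP_GhostEnemy and BP_Clown actors, with debug prints.
; EnableSwordDamage and DisableSwordDamage toggle hitbox collision so outside callers can control when hits register.
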(event `self.Sphere.OnComponentBeginOverlap`
  (params (OverlappedComponent :type "PrimitiveComponent Object Reference") (OtherActor :type "Actor Object Reference") (OtherComp :type "PrimitiveComponent Object Reference") (OtherBodyIndex :type Integer) (bFromSweep :type Boolean) (SweepResult :type "HitResult Structure (by ref)"))
  (bind _asbp_third_person_character (cast `/Game/ThirdPerson/Blueprints/BP_ThirdPersonCharacter` OtherActor))
  (set `/Game/ThirdPerson/Blueprints/BP_ThirdPersonCharacter.SwordRef` self _asbp_third_person_character)
  (`SceneComponent.K2_AttachToComponent` (`self.StaticMesh`) (`Character.Mesh` _asbp_third_person_character) "SwordSocket" "SnapToTarget" "SnapToTarget" "KeepWorld" true)
  (set `/Game/ThirdPerson/Blueprints/BP_ThirdPersonCharacter.HasSword` true _asbp_third_person_character))

(event `self.SwordHitbox.OnComponentBeginOverlap`
  (params (OverlappedComponent :type "PrimitiveComponent Object Reference") (OtherActor :type "Actor Object Reference") (OtherComp :type "PrimitiveComponent Object Reference") (OtherBodyIndex :type Integer) (bFromSweep :type Boolean) (SweepResult :type "HitResult Structure (by ref)"))
  (`|ExecutionSequence`
    (:`then_0`
      (bind _asbp_ghost_enemy (cast `/Game/BP_GhostEnemy` OtherActor))
      (`KismetSystemLibrary.PrintString` "hit")
      (`GameplayStatics.ApplyDamage` _asbp_ghost_enemy 10.0 null (`self.GetOwner`)))
    (:`then_1`
      (bind _asbp_clown (cast `/Game/ClownEnemy/BP_Clown` OtherActor))
      (`KismetSystemLibrary.PrintString` "Hit")
      (`GameplayStatics.ApplyDamage` _asbp_clown 10.0))))

(fn `DisableSwordDamage`
  (`PrimitiveComponent.SetCollisionEnabled` (`self.SwordHitbox`) "NoCollision"))

(fn `EnableSwordDamage`
  (`PrimitiveComponent.SetCollisionEnabled` (`self.SwordHitbox`) "QueryOnly"))

(fn `UserConstructionScript`)