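; BP_TunnelGate is a progress-locked gate that starts the clown boss encounter when the third-person player enters its trigger.
; The overlap checks kill and objective-item counts, printing a "not ready" message if either falls short.
; On success it destroys the gate mesh, plays the boss intro, then blends the view back to the player after a delay.
; It then enables the clown's walking and chasing and removes the trigger.
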(event `self.GateTrigger.OnComponentBeginOverlap`
  (params (OverlappedComponent :type "PrimitiveComponent Object Reference") (OtherActor :type "Actor Object Reference") (OtherComp :type "PrimitiveComponent Object Reference") (OtherBodyIndex :type Integer) (bFromSweep :type Boolean) (SweepResult :type "HitResult Structure (by ref)"))
  (bind _asbp_third_person_character (cast `/Game/ThirdPerson/Blueprints/BP_ThirdPersonCharacter` OtherActor))
  (if (and (>= (`/Game/ThirdPerson/Blueprints/BP_ThirdPersonCharacter.EnemiesKilled` _asbp_third_person_character) 20) (>= (`/Game/ThirdPerson/Blueprints/BP_ThirdPersonCharacter.ObjectiveItemsCollected` _asbp_third_person_character) 1))
    (`ActorComponent.K2_DestroyComponent` (`self.GateMesh`))
    (`PlayerController.SetViewTargetWithBlend` (`GameplayStatics.GetPlayerController` 0) null 2.0 "VTBlend_Linear" 0.0 false)
    (`/Game/ClownEnemy/BP_Clown.PlayBossIntro` (`self.ClownRef`))
    (`KismetSystemLibrary.Delay` 2.0)
    (bind _returnvalue (`InputDeviceLibrary.GetPlayerControllerFromPlatformUser` (struct)))
    (`PlayerController.SetViewTargetWithBlend` _returnvalue (`GameplayStatics.GetPlayerCharacter` 0) 2.0 "VTBlend_Linear" 0.0 false)
    (`CharacterMovementComponent.SetMovementMode` (`Character.CharacterMovement` (`self.ClownRef`)) "MOVE_Walking" 0)
    (set `/Game/ClownEnemy/BP_Clown.CanChasePlayer` true (`self.ClownRef`))
    (`ActorComponent.K2_DestroyComponent` (`self.GateTrigger`))
    (else
      (`KismetSystemLibrary.PrintString` "The stage is not ready for you yet..."))))

(fn `UserConstructionScript`)