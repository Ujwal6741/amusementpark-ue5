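; Enemy spawner actor that periodically spawns BP_GhostEnemy instances at its own transform.
; On BeginPlay it starts a looping timer that fires a spawn event at a fixed interval.
; Each spawn increments a running counter, and once that count reaches MaxEnemies the timer is cleared.
; The count never decreases here, so the cap limits total spawns rather than enemies alive.
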(event `self.ReceiveBeginPlay`
  (bind _returnvalue (`KismetSystemLibrary.K2_SetTimerDelegate` (delegate `SpawnEnemy`) 3.0 true))
  (set `self.SpawnTimerHandle` _returnvalue))

(event `SpawnEnemy`
  (if (< (`self.SpawnedEnemies`) (`self.MaxEnemies`))
    (`|SpawnActorFromClass` "/Game/BP_GhostEnemy.BP_GhostEnemy_C" (`self.GetTransform`) "Undefined" "MultiplyWithRoot" null null)
    (set `self.SpawnedEnemies` (+ (`self.SpawnedEnemies`) 1))
    (else
      (`KismetSystemLibrary.K2_ClearAndInvalidateTimerHandle` (`self.SpawnTimerHandle`)))))

(fn `UserConstructionScript`)